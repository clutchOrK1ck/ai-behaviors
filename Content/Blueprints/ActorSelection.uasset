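; ActorSelection maintains a list of selected actors and exposes functions to add, remove, toggle, replace, query and clear it.
; Add stores each valid actor once, and Set clears the current selection before adding the given actor.
; Add, Remove and Clear update each actor's SelectableComponent through SetSelected, keeping its selected state in step with the list.
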(fn `Add`
  (params (Actor :type "Actor Object Reference"))
  (bind _returnvalue (`Actor.GetComponentByClass` Actor "/Game/Blueprints/SelectableComponent.SelectableComponent_C"))
  (`/Engine/EditorBlueprintResources/StandardMacros.IsValid` Actor
    (:`Is Valid`
      (`KismetArrayLibrary.Array_AddUnique` (`self.Selection`) Actor)
      (`/Engine/EditorBlueprintResources/StandardMacros.IsValid` _returnvalue
        (:`Is Valid`
          (`/Game/Blueprints/SelectableComponent.SetSelected` _returnvalue true))))))

(fn `Clear`
  (bind _selection (`self.Selection`))
  (for _array_element _selection
    (`/Engine/EditorBlueprintResources/StandardMacros.IsValid` _array_element
      (:`Is Valid`
        (bind _returnvalue (`Actor.GetComponentByClass` _array_element "/Game/Blueprints/SelectableComponent.SelectableComponent_C"))
        (`/Engine/EditorBlueprintResources/StandardMacros.IsValid` _returnvalue
          (:`Is Valid`
            (`/Game/Blueprints/SelectableComponent.SetSelected` _returnvalue false))))))
  (`KismetArrayLibrary.Array_Clear` _selection))

(fn `Contains`
  (params (Actor :type "Actor Object Reference"))
  (returns (Result :type Boolean))
  (return (`KismetArrayLibrary.Array_Contains` (`self.Selection`) Actor)))

(fn `IsEmpty`
  (returns (Result :type Boolean))
  (return (`KismetArrayLibrary.Array_IsEmpty` (`self.Selection`))))

(fn `Remove`
  (params (Actor :type "Actor Object Reference"))
  (bind _returnvalue (`Actor.GetComponentByClass` Actor "/Game/Blueprints/SelectableComponent.SelectableComponent_C"))
  (bind _returnvalue_2 (`KismetArrayLibrary.Array_RemoveItem` (`self.Selection`) Actor))
  (if _returnvalue_2
    (`/Engine/EditorBlueprintResources/StandardMacros.IsValid` _returnvalue
      (:`Is Valid`
        (`/Game/Blueprints/SelectableComponent.SetSelected` _returnvalue false)))))

(fn `Set`
  (params (Actor :type "Actor Object Reference"))
  (if (`KismetArrayLibrary.Array_IsNotEmpty` (`self.Selection`))
    (`self.Clear`))
  (`self.Add` Actor))

(fn `Toggle`
  (params (Actor :type "Actor Object Reference"))
  (if (`KismetArrayLibrary.Array_Contains` (`self.Selection`) Actor)
    (`self.Remove` Actor)
    (else
      (`self.Add` Actor))))