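; Navigation path visualizer actor that marks each point of a path with a mesh instance.
; Its Update event clears all five instanced mesh components, then rebuilds them from the supplied path points.
; Each point type selects a component: waypoint, navlink in, navlink out, off-mesh waypoint or destination, with bidirectional navlinks sharing the in marker.
; Instances are placed in world space, unrotated and at unit scale.
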(event `self.Update`
  (params (PathPoints :type "Array of PathVisPathPoint Structure (by ref)"))
  (`self.RebuildVisualization` PathPoints))

(fn `AddVisInstance`
  (params (Location :type "Vector Structure") (Meshes :type "InstancedStaticMeshComponent Object Reference"))
  (`InstancedStaticMeshComponent.AddInstance` Meshes (`KismetMathLibrary.MakeTransform` Location) true))

(fn `ClearVisInstances`
  (for _array_element (`|MakeArray` (`self.WaypointVisMeshes`) (`self.NavLinkInVisMeshes`) (`self.OffMeshVisMeshes`) (`self.DestinationVisMeshes`) (`self.NavLinkOutVisMeshes`))
    (`InstancedStaticMeshComponent.ClearInstances` _array_element)))

(fn `RebuildVisualization`
  (params (Locations :type "Array of PathVisPathPoint Structure"))
  (`self.ClearVisInstances`)
  (for _array_element Locations
    (switch `EPathVisualizationPointType` (`.Type` (break `PathVisPathPoint` _array_element))
      (:`Waypoint`
        (`self.AddVisInstance` (break `PathVisPathPoint` _array_element) (`self.WaypointVisMeshes`)))
      (:`NavlinkStart`
        (`self.AddVisInstance` (break `PathVisPathPoint` _array_element) (`self.NavLinkInVisMeshes`) :!label _label))
      (:`NavlinkEnd`
        (`self.AddVisInstance` (break `PathVisPathPoint` _array_element) (`self.NavLinkOutVisMeshes`)))
      (:`NavlinkBi`
        (goto _label))
      (:`OffMeshWaypoint`
        (`self.AddVisInstance` (break `PathVisPathPoint` _array_element) (`self.OffMeshVisMeshes`)))
      (:`Destination`
        (`self.AddVisInstance` (break `PathVisPathPoint` _array_element) (`self.DestinationVisMeshes`))))))

(fn `UserConstructionScript`)