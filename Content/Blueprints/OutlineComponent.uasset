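; Actor component that outlines its owner on cursor hover and selection through custom depth stencil values.
; On BeginPlay it binds to the owner's cursor-over events and, if present, the select and deselect events of its SelectableComponent.
; Changes write the stencil ID to every primitive component on the owner, with custom depth enabled.
; Selection uses its own ID and suspends hover handling until deselection.
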(event `OnBeginCursorOver_Event`
  (params (TouchedActor :type "Actor Object Reference"))
  ; Bind to begin cursor hover
  (if (`self.ProcessMouseOverEvents`)
    (`self.SetStencilId` (`self.DefaultStencilId`))))

(event `self.ReceiveBeginPlay`
  (bind _returnvalue (`Actor.GetComponentByClass` (`self.GetOwner`) "/Game/Blueprints/SelectableComponent.SelectableComponent_C"))
  (bind _returnvalue_2 (`Actor.GetComponentByClass` (`self.GetOwner`) "/Game/Blueprints/SelectableComponent.SelectableComponent_C"))
  (`|ExecutionSequence`
    (:`then_0`
      ; Bind to begin cursor hover
      (add `Actor.OnBeginCursorOver` (`self.GetOwner`) (delegate `OnBeginCursorOver_Event`)))
    (:`then_1`
      ; Bind to end cursor hover
      (add `Actor.OnEndCursorOver` (`self.GetOwner`) (delegate `OnEndCursorOver_Event`)))
    (:`then_2`
      ; Draw outline on selection
      (`/Engine/EditorBlueprintResources/StandardMacros.IsValid` _returnvalue_2
        (:`Is Valid`
          (add `/Game/Blueprints/SelectableComponent.OnActorSelected` _returnvalue_2 (delegate `DrawSelectionOutline`)))))
    (:`then_3`
      ; Remove outline on deselection
      (`/Engine/EditorBlueprintResources/StandardMacros.IsValid` _returnvalue
        (:`Is Valid`
          (add `/Game/Blueprints/SelectableComponent.OnActorDeselected` _returnvalue (delegate `RemoveSelectionOutline`)))))))

(event `OnEndCursorOver_Event`
  (params (TouchedActor :type "Actor Object Reference"))
  ; Bind to end cursor hover
  (if (`self.ProcessMouseOverEvents`)
    (`self.SetStencilId` 0)))

(event `DrawSelectionOutline`
  ; Draw outline on selection
  (set `self.ProcessMouseOverEvents` false)
  (`self.SetStencilId` 3))

(event `RemoveSelectionOutline`
  ; Remove outline on deselection
  (set `self.ProcessMouseOverEvents` true)
  (`self.SetStencilId` 0))

(fn `SetStencilId`
  (params (Id :type Integer))
  (for _array_element (`Actor.K2_GetComponentsByClass` (`self.GetOwner`) "/Script/Engine.PrimitiveComponent")
    (`self.SetStencilIdForComponent` _array_element Id)))

(fn `SetStencilIdForComponent`
  (params (Component :type "PrimitiveComponent Object Reference") (Id :type Integer))
  (`PrimitiveComponent.SetRenderCustomDepth` Component true)
  (`PrimitiveComponent.SetCustomDepthStencilValue` Component Id))