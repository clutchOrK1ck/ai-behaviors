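; SceneCamera is a spring-arm camera rig that orbits, elevates and zooms around its pivot through three input functions, all scaled by delta time.
; Yaw input rotates the arm, and zoom input changes its length.
; Elevation offsets the camera position along world Z, then derives arm pitch (via AngleBetween, scaled by negated input) and new length from that target.
; The event graph is empty, so callers must supply the input.
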(fn `AddElevationInput`
  (params (ElevationInput :type "Float (double-precision)"))
  (locals (CameraPivotToActorRootLocation :type "Vector Structure") (TargetCameraToActorLocation :type "Vector Structure") (Displacement :type "Vector Structure") (lclElevation :type "Float (double-precision)") (ElevationDelta :type "Float (double-precision)" :default 0.0))
  (bind _springarm (`self.SpringArm`))
  (set `local.lclElevation` ElevationInput)
  (set `local.ElevationDelta` (* (* ElevationInput (`self.ElevationChangeRate`)) (`GameplayStatics.GetWorldDeltaSeconds`)))
  (set `local.Displacement` (`KismetMathLibrary.MakeVector` 0.0 0.0 (`local.ElevationDelta`)))
  (set `local.CameraPivotToActorRootLocation` (* (* (`SceneComponent.GetForwardVector` (`self.SpringArm`)) -1.0) (`SpringArmComponent.TargetArmLength` (`self.SpringArm`))))
  (set `local.TargetCameraToActorLocation` (+ (`local.CameraPivotToActorRootLocation`) (`local.Displacement`)))
  (`SceneComponent.K2_AddLocalRotation` _springarm (`KismetMathLibrary.MakeRotator` 0.0 (* (`self.AngleBetween` (`local.CameraPivotToActorRootLocation`) (`local.TargetCameraToActorLocation`)) (* (`local.lclElevation`) -1.0))) false false)
  (set `SpringArmComponent.TargetArmLength` (`KismetMathLibrary.VSize` (`local.TargetCameraToActorLocation`)) _springarm))

(fn `AddYawInput`
  (params (Yaw :type "Float (double-precision)"))
  (`SceneComponent.K2_AddRelativeRotation` (`self.SpringArm`) (`KismetMathLibrary.MakeRotator` 0.0 0.0 (* (* (* Yaw -1.0) (`self.RotationSpeed`)) (`GameplayStatics.GetWorldDeltaSeconds`))) false false))

(fn `AddZoomInput`
  (params (Zoom :type "Float (double-precision)"))
  (bind _springarm (`self.SpringArm`))
  (set `SpringArmComponent.TargetArmLength` (- (`SpringArmComponent.TargetArmLength` _springarm) (* (* (`self.ZoomSpeed`) Zoom) (`GameplayStatics.GetWorldDeltaSeconds`))) _springarm))

(fn `AngleBetween`
  (params (A :type "Vector Structure") (B :type "Vector Structure"))
  (returns (`Angle (Degrees)` :type "Float (double-precision)"))
  (return (`KismetMathLibrary.DegAcos` (/ (`KismetMathLibrary.Dot_VectorVector` A B) (* (`KismetMathLibrary.VSize` A) (`KismetMathLibrary.VSize` B))))))

(fn `UserConstructionScript`)