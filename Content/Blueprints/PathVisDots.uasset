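; PathVisDots visualizes navigation paths as dots through a separate NavPathDotVisualization actor.
; RedrawPathVisualization passes incoming path points to that actor to rebuild the display, or destroys the actor when the point list is empty.
; GetCreatePathVisActor lazily spawns the actor at the owner's transform and caches it for reuse on later redraws.
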(fn `GetCreatePathVisActor`
  (returns (PathVisActor :type "/Game/Blueprints/NavPathDotVisualization Object Reference"))
  (`/Engine/EditorBlueprintResources/StandardMacros.IsValid` (`self.PathVisActor`)
    (:`Is Valid`
      (return (`self.PathVisActor`)))
    (:`Is Not Valid`
      (bind _returnvalue (`|SpawnActorFromClass` "/Game/Blueprints/NavPathDotVisualization.NavPathDotVisualization_C" (`Actor.GetTransform` (`self.GetOwner`)) "AlwaysSpawn" "MultiplyWithRoot" null 5.0 (struct) null))
      (bind _output_get (set `self.PathVisActor` _returnvalue))
      (return _output_get))))

(fn `RedrawPathVisualization`
  (params (InPathPoints :type "Array of PathVisPathPoint Structure (by ref)"))
  (bind _pathvisactor (`self.PathVisActor`))
  (if (`KismetArrayLibrary.Array_IsEmpty` InPathPoints)
    (`/Engine/EditorBlueprintResources/StandardMacros.IsValid` _pathvisactor
      (:`Is Valid`
        (`Actor.K2_DestroyActor` _pathvisactor)))
    (else
      (`/Game/Blueprints/NavPathDotVisualization.RebuildVisualization` (`self.GetCreatePathVisActor`) InPathPoints)))
  (return))